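; BP_ChamferCube is a flammable cube that can catch, spread and lose fire.
; On BeginPlay it registers with BP_ThirdPersonGameMode as flammable and randomly starts burning or unlit.
; AddFire accumulates heat until BurnThreshold ignites it, while Interact or Douse extinguishes it and clears the amount.
; SetFireState toggles the fire effect and spreader component together, and IsOnFire reads the effect's visibility as the burning state.
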(event EventAddFire
  (params (Amount :type Float%20%28double-precision%29))
  (bind _output_get (Variables|Default|SetCurrentFireAmount (+ Amount (Variables|Default|GetCurrentFireAmount))))
  (if (>= _output_get (Variables|Default|GetBurnThreshold))
    (CallFunction|SetFireState true)))

(event EventInteract
  (CallFunction|Douse))

(event EventDouse
  (CallFunction|SetFireState false))

(event EventBeginPlay
  (bind _asbp_third_person_game_mode (Utilities|Casting|CastToBP_ThirdPersonGameMode (Game|GetGameMode)))
  (Default|RegisterFlammable _asbp_third_person_game_mode self)
  (CallFunction|SetFireState (Math|Random|RandomBool)))

(fn ConstructionScript)

(fn SetFireState
  (params (FireActive :type Boolean))
  (if FireActive
    _
    (else
      (Variables|Default|SetCurrentFireAmount 0.0)))
  (Rendering|SetVisibility (Variables|Default|GetP_Fire) FireActive false)
  (Components|Activation|SetActive (Variables|Default|GetAC_FireSpreader) FireActive false))

(fn IsonFire
  (return (Rendering|IsVisible (Variables|Default|GetP_Fire))))