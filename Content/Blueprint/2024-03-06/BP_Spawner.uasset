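; BP_Spawner is a spawner actor that scatters randomly chosen actors around its location when play begins.
; A BeginPlay loop spawns SpawnCount actors, each picked at random from SpawnedActor, and stores them in SpawnedInstances.
; Positions come from random unit vectors scaled by SpawnRadius with Z zeroed, and collision handling adjusts placement but always spawns.
; Tick draws a debug sphere showing the radius, purely as a visual aid.
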(event EventBeginPlay
  (bind _returnvalue (Math|Random|RandomUnitVector))
  (bind _spawnradius (Variables|Default|GetSpawnRadius))
  (bind _returnvalue_2 (* _returnvalue _spawnradius))
  (for _index (range 0 (- (Variables|Default|GetSpawnCount) 1))
    (bind _returnvalue_3 (Game|SpawnActorfromClass (.OutItem (Utilities|Array|Random (Variables|Default|GetSpawnedActor))) (Math|Transform|MakeTransform (+ (Transformation|GetActorLocation) (Math|Vector|MakeVector (.x _returnvalue_2) (.y _returnvalue_2) 0.0))) "AdjustIfPossibleButAlwaysSpawn" "MultiplyWithRoot" 0 0))
    (Utilities|Array|Add (Variables|Default|GetSpawnedInstances) _returnvalue_3)))

(event EventTick
  (params (DeltaSeconds :type Float%20%28single-precision%29))
  ;[1 1 1] Not necessary - only for debug visuals
  (Rendering|Debug|DrawDebugSphere (Transformation|GetActorLocation) (Variables|Default|GetSpawnRadius) 12 "(R=1.000000,G=1.000000,B=1.000000,A=1.000000)" 0.0 25.0))

(fn ConstructionScript)