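; Test actor that renders a line as a procedural mesh quad, shortened where a trace from the actor hits something.
; BeginPlay creates a two-triangle mesh section with the M_LineRender material.
; Each Tick traces forward on Visibility up to CurrentLength, then passes the hit distance or full length as local X to UpdateLineMesh.
; That function appends four corners offset by HalfWidth along the actor's up vector and updates the section.
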(event EventTick
  (params (DeltaSeconds :type Float%20%28single-precision%29))
  (bind _returnvalue (Transformation|GetActorLocation))
  (bind _outhit (Collision|LineTraceByChannel _returnvalue (+ _returnvalue (* (Transformation|GetActorForwardVector) (Variables|Default|GetCurrentLength))) "TraceTypeQuery1" false 0 "ForOneFrame"))
  (if (.bblockinghit _outhit)
    (CallFunction|UpdateLineMesh "0, 0, 0" (Math|Vector|MakeVector (.distance _outhit) 0.0 0.0))
    (else
      (CallFunction|UpdateLineMesh "0, 0, 0" (Math|Vector|MakeVector (Variables|Default|GetCurrentLength) 0.0 0.0)))))

(event EventBeginPlay
  (CallFunction|GenerateLineMesh))

(fn ConstructionScript)

(fn GenerateLineMesh
  (bind _triangles (LocalVariables|GetTriangles))
  (bind _proceduralmesh (Variables|Default|GetProceduralMesh))
  ;[1 1 1] First Triangle
  (Utilities|Array|Add _triangles 0)
  (Utilities|Array|Add _triangles 1)
  (Utilities|Array|Add _triangles 2)
  ;[1 1 1] Second Triangle
  (Utilities|Array|Add _triangles 2)
  (Utilities|Array|Add _triangles 3)
  (Utilities|Array|Add _triangles 0)
  (Class|ProceduralMeshComponent|CreateMeshSectionLinearColor _proceduralmesh 0 (LocalVariables|GetVertices) (LocalVariables|GetTriangles) 0 0 0 0 0 0 0 false false)
  (Rendering|Material|SetMaterial _proceduralmesh 0 "/Game/Blueprint/2024-03-27/M_LineRender.M_LineRender"))

(fn UpdateLineMesh
  (params (Origin :type Vector) (Target :type Vector))
  (bind _returnvalue (Transformation|GetActorUpVector))
  (bind _vertices (LocalVariables|GetVertices))
  ;[1 1 1] Upwards Offset for Vertex 0
  (Utilities|Array|Add _vertices (+ Origin (* _returnvalue (Variables|Default|GetHalfWidth))))
  ;[1 1 1] Downwards Offset for Vertex 1
  (Utilities|Array|Add _vertices (+ Origin (* _returnvalue (* (Variables|Default|GetHalfWidth) -1.0))))
  ;[1 1 1] Forwards and Downwards Offsets for Vertex 2
  (Utilities|Array|Add _vertices (+ Target (* (Transformation|GetActorUpVector) (* (Variables|Default|GetHalfWidth) -1.0))))
  ;[1 1 1] Forwards and Upwards Offset for Vertex 3
  (Utilities|Array|Add _vertices (+ Target (* (Transformation|GetActorUpVector) (Variables|Default|GetHalfWidth))))
  (Class|ProceduralMeshComponent|UpdateMeshSectionLinearColor (Variables|Default|GetProceduralMesh) 0 (LocalVariables|GetVertices) 0 0 0 0 0 0 0 true))