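; BP_InteractiveActor is an actor that can be interacted with and set on fire.
; Its construction script makes the Sphere block a custom trace channel, GameTraceChannel1.
; Interact only prints a debug string, while AddFire accumulates FireAmount and shows the PFire component once it reaches BurnThreshold.
; IsOnFire reads the burning state straight from PFire's visibility, and nothing here reduces the fire or hides it again.
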(event EventInteract
  (Development|PrintString "Interacted!!!"))

(event EventAddFire
  (params (Amount :type Float%20%28double-precision%29))
  (bind _output_get (Variables|Default|SetFireAmount (+ (Variables|Default|GetFireAmount) Amount)))
  (if (>= _output_get (Variables|Default|GetBurnThreshold))
    (Rendering|SetVisibility (Variables|Default|GetP_Fire) true false)))

(fn ConstructionScript
  (Collision|SetCollisionResponsetoChannel (Variables|Default|GetSphere) "ECC_GameTraceChannel1" "ECR_Block"))

(fn IsonFire
  (return (Rendering|IsVisible (Variables|Default|GetP_Fire))))