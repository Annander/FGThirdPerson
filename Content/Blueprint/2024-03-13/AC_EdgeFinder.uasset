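; AC_EdgeFinder is an actor component that looks for a ledge or drop-off ahead of its owner every tick.
; It steps along the owner's forward vector up to Reach in StepLength increments, tracing vertically downward through each point on the Visibility channel.
; The first missed trace marks an edge at the last hit location, which Tick shows as a pink debug point.
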(event EventTick
  (params (DeltaSeconds :type Float%20%28single-precision%29))
  (bind (_edgedetected _edge) (CallFunction|EdgeDetect))
  (if _edgedetected
    (Rendering|Debug|DrawDebugPoint _edge 1e+02 "(R=1.000000,G=0.000000,B=0.578816,A=1.000000)" 0.0)))

(fn EdgeDetect
  (LocalVariables|SetCheck 0.0)
  (LocalVariables|SetOwner (Components|GetOwner))
  (while (<= (LocalVariables|GetCheck) (Variables|Default|GetReach))
    (bind (_outhit _returnvalue) (Collision|LineTraceByChannel (+ (+ (Transformation|GetActorLocation (LocalVariables|GetOwner)) (* (Transformation|GetActorForwardVector (LocalVariables|GetOwner)) (LocalVariables|GetCheck))) (* (Math|Vector|VectorUp) 5e+02)) (+ (+ (+ (Transformation|GetActorLocation (LocalVariables|GetOwner)) (* (Transformation|GetActorForwardVector (LocalVariables|GetOwner)) (LocalVariables|GetCheck))) (* (Math|Vector|VectorUp) 5e+02)) (* (Math|Vector|VectorDown) 1e+03)) "TraceTypeQuery1" false 0 "ForOneFrame"))
    (LocalVariables|SetCheck (+ (LocalVariables|GetCheck) (Variables|Default|GetStepLength)))
    (if _returnvalue
      (bind _output_get (LocalVariables|SetPreviousHitResult _outhit))
      (else
        (return true (.Location (Collision|BreakHitResult _output_get))))))
  (return false "0, 0, 0"))