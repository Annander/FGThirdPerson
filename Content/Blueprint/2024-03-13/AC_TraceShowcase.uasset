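; AC_TraceShowcase is an actor component that demonstrates trace types by drawing them from its owning actor.
; Every tick it switches on TraceType to run a single or multi line or sphere trace by channel along the owner's forward vector.
; TraceDistance, TraceChannel and Radius shape the trace, which is debug-drawn for one frame, and its hit results go unused.
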(event EventTick
  (params (DeltaSeconds :type Float%20%28single-precision%29))
  (bind _returnvalue (Components|GetOwner))
  (bind _tracedistance (Variables|Default|GetTraceDistance))
  (bind _radius (Variables|Default|GetRadius))
  (bind _trace_channel (Variables|Default|GetTrace%20Channel))
  (bind _returnvalue_2 (Transformation|GetActorLocation _returnvalue))
  (bind _returnvalue_3 (Transformation|GetActorForwardVector _returnvalue))
  (bind _returnvalue_4 (* _returnvalue_3 _tracedistance))
  (bind _returnvalue_5 (+ _returnvalue_2 _returnvalue_4))
  (switch Utilities|FlowControl|Switch|SwitchonE_TraceType (Variables|Default|GetTraceType)
    (:NewEnumerator0
      (Collision|LineTraceByChannel _returnvalue_2 _returnvalue_5 _trace_channel false 0 "ForOneFrame"))
    (:NewEnumerator1
      (Collision|MultiLineTraceByChannel _returnvalue_2 _returnvalue_5 _trace_channel false 0 "ForOneFrame"))
    (:NewEnumerator2
      (Collision|SphereTraceByChannel _returnvalue_2 _returnvalue_5 _radius _trace_channel false 0 "ForOneFrame"))
    (:NewEnumerator3
      (Collision|MultiSphereTraceByChannel _returnvalue_2 _returnvalue_5 _radius _trace_channel false 0 "ForOneFrame"))))