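; BP_PhysicsEvents is a debug or demonstration actor that shows when a Cube component's physics and collision events fire.
; The event graph binds the Cube's hit, begin and end overlap, wake, sleep and physics state change events, each printing a label on screen.
; The state change handler also appends the enum value as text, and the construction script is empty.
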(event OnComponentHit(Cube)
  (params (HitComponent :type Primitive%20Component%20Object%20Reference) (OtherActor :type Actor%20Object%20Reference) (OtherComp :type Primitive%20Component%20Object%20Reference) (NormalImpulse :type Vector :default "0, 0, 0") (Hit :type Hit%20Result%20Structure%20%28by%20ref%29))
  (Development|PrintString "Hit"))

(event OnComponentBeginOverlap(Cube)
  (params (OverlappedComponent :type Primitive%20Component%20Object%20Reference) (OtherActor :type Actor%20Object%20Reference) (OtherComp :type Primitive%20Component%20Object%20Reference) (OtherBodyIndex :type Integer) (bFromSweep :type Boolean) (SweepResult :type Hit%20Result%20Structure%20%28by%20ref%29))
  (Development|PrintString "Begin Overlap"))

(event OnComponentEndOverlap(Cube)
  (params (OverlappedComponent :type Primitive%20Component%20Object%20Reference) (OtherActor :type Actor%20Object%20Reference) (OtherComp :type Primitive%20Component%20Object%20Reference) (OtherBodyIndex :type Integer))
  (Development|PrintString "End Overlap"))

(event OnComponentWake(Cube)
  (params (WakingComponent :type Primitive%20Component%20Object%20Reference) (BoneName :type Name :default "None"))
  (Development|PrintString "Component Wake"))

(event OnComponentSleep(Cube)
  (params (SleepingComponent :type Primitive%20Component%20Object%20Reference) (BoneName :type Name :default "None"))
  (Development|PrintString "Component Sleep"))

(event OnComponentPhysicsStateChanged(Cube)
  (params (ChangedComponent :type Primitive%20Component%20Object%20Reference) (StateChange :type EComponentPhysicsStateChange%20Enum :default "Created"))
  (Development|PrintString (Utilities|String|Append "State Changed: " (Utilities|String|EnumtoString StateChange))))

(fn ConstructionScript)