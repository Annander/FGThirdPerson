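; Interactor component for the third-person character that finds the object under the camera's aim and interacts with it.
; Every tick a debug-drawn multi line trace from the follow camera picks the closest hit, sending become/stop-candidate messages as the target changes.
; Interact sends an interact message to the current target.
; It also prints on the character's fire-spawned event and provides a downward-trace helper returning a capsule-height ground position.
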(event Custom|OnFireSpawned
  (Development|PrintString "Interactor acknowledged a spawned fire!"))

(event EventTick
  (params (DeltaSeconds :type Float%20%28single-precision%29))
  (bind _as_bp_third_person_character (Variables|Default|GetAs%20BP%20Third%20Person%20Character))
  (bind _followcamera (Variables|/Game/ThirdPerson/Blueprints/BP_ThirdPersonCharacter.BP_ThirdPersonCharacter_C|GetFollowCamera _as_bp_third_person_character))
  (bind _returnvalue (Transformation|GetWorldLocation _followcamera))
  (bind _output_get (Variables|Default|SetLastFrameTarget (Variables|Default|GetCurrentTarget)))
  (Variables|Default|SetCurrentTarget 0)
  (bind (_outhits _returnvalue_2) (Collision|MultiLineTraceByChannel _returnvalue (+ _returnvalue (* (Math|Vector|GetForwardVector _followcamera) 1e+18)) "TraceTypeQuery3" false (Utilities|Array|MakeArray _as_bp_third_person_character) "ForOneFrame"))
  (if _returnvalue_2
    (bind _output_get_2 (Variables|Default|SetClosestDistance 1e+18))
    (for _array_element _outhits
      (Math|Float|CompareFloat (Math|Vector|Distance(Vector) _returnvalue (.location _array_element)) _output_get_2
        (:<
          (Variables|Default|SetClosestDistance (Math|Vector|Distance(Vector) _returnvalue (.location _array_element)))
          (bind _output_get_3 (Variables|Default|SetCurrentTarget (.hitactor _array_element)))
          (if (not (== (Variables|Default|GetLastFrameTarget) _output_get_3))
            (Class|BIInteractable|OnBecomeCandidate(Message) _output_get_3)
            (Class|BIInteractable|OnStopBeingACandidate(Message) (Variables|Default|GetLastFrameTarget))))))
    (else
      (Class|BIInteractable|OnStopBeingACandidate(Message) _output_get))))

(event EventBeginPlay
  (bind _asbp_third_person_character (Utilities|Casting|CastToBP_ThirdPersonCharacter (Components|GetOwner)))
  (Variables|Default|SetAs%20BP%20Third%20Person%20Character _asbp_third_person_character)
  (EventDispatchers|BindEventtoOnFireSpawned _asbp_third_person_character (delegate Custom|OnFireSpawned)))

(fn Interact
  (bind _currenttarget (Variables|Default|GetCurrentTarget))
  (Utilities|IsValid _currenttarget
    (:Is%20Valid
      (Class|BIInteractable|Interact(Message) _currenttarget))))

(fn FindGroundOffset
  (params (Target :type Actor%20Object%20Reference) (CapsuleHalfHeight :type Float%20%28double-precision%29))
  (bind _returnvalue (Transformation|GetActorLocation Target))
  (bind _outhit (Collision|LineTraceByChannel _returnvalue (+ _returnvalue (* (Math|Vector|VectorDown) 128.0)) "TraceTypeQuery1" false 0 "None"))
  (return (+ (.Location (Collision|BreakHitResult _outhit)) (* (.Normal (Collision|BreakHitResult _outhit)) CapsuleHalfHeight))))