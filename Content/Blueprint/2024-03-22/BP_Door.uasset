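; BP_Door is an interactable door that slides its Cube by a Destination offset from the location cached in the construction script.
; Interact starts a one-shot timer unless one is running, and Tick feeds its normalized elapsed time through a Curve to drive the lerp.
; Timer completion toggles Open and brightens a point light when true.
; The motion always plays from start toward Destination, regardless of Open.
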(event Custom|OnTimerCompleted
  (bind _output_get (Variables|Default|SetOpen (not (Variables|Default|GetOpen))))
  (if _output_get
    (Rendering|Components|Light|SetIntensity (Variables|Default|GetPointLight) 5e+03)))

(event EventInteract
  (if (not (Utilities|Time|IsTimerActivebyHandle (Variables|Default|GetTimerHandle)))
    (bind _returnvalue (Utilities|Time|SetTimerbyEvent (delegate Custom|OnTimerCompleted) (Variables|Default|GetDuration)))
    (Variables|Default|SetTimerHandle _returnvalue)))

(event EventTick
  (params (DeltaSeconds :type Float%20%28single-precision%29))
  (bind _timerhandle (Variables|Default|GetTimerHandle))
  (if (Utilities|Time|IsTimerActivebyHandle _timerhandle)
    (Transformation|SetRelativeLocation (Variables|Default|GetCube) (+ (Variables|Default|GetRelative%20Location) (Math|Vector|Lerp(Vector) "0, 0, 0" (Variables|Default|GetDestination) (Math|Curves|GetFloatValue (Variables|Default|GetCurve) (/ (Class|KismetSystemLibrary|GetTimerElapsedTimeHandle _timerhandle) (Variables|Default|GetDuration))))) false false)))

(fn ConstructionScript
  (Variables|Default|SetRelative%20Location (Variables|/Script/Engine.SceneComponent|GetRelativeLocation (Variables|Default|GetCube))))